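; BP_PlayerTank is the player-controlled tank, wiring input to movement, camera and firing.
; Each tick it passes the forward and turning axis values to the TankMovement component's HandleTankMovement.
; Turn input yaws CameraRoot, while LookUp pitches the SpringArm within a clamped range, separating orbit yaw from pitch.
; Pressing Fire calls Fire on the TankAiming component.
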(event EventBeginPlay
  (|CallParentFunction) ; This node is disabled and will not be called.\nDrag off pins to build functionality.
)

(event Collision|EventActorBeginOverlap
  (params (OtherActor :type Actor%20Object%20Reference))
  (|CallParentFunction OtherActor) ; This node is disabled and will not be called.\nDrag off pins to build functionality.
)

(event EventTick
  (params (DeltaSeconds :type Float%20%28single-precision%29))
  (|CallParentFunction DeltaSeconds)
  (Class|TankMovementComponent|HandleTankMovement (Variables|Default|GetTankMovement) (Input|AxisValues|GetMoveForward) (Input|AxisValues|GetMoveTurning)))

(event Input|ActionEvents|InputActionFire
  (params (Key :type Key%20Structure))
  (:Pressed
    (Class|TankAimingComponent|Fire (Variables|Default|GetTankAiming))))

(event Input|AxisEvents|InputAxisLookUp
  (params (AxisValue :type Float%20%28single-precision%29))
  (bind _springarm (Variables|Default|GetSpringArm))
  (bind _relativerotation (Variables|/Script/Engine.SceneComponent|GetRelativeRotation _springarm))
  (Transformation|SetRelativeRotation _springarm (Math|Rotator|MakeRotator (.roll _relativerotation) (Math|Float|Clamp(Float) (+ AxisValue (.pitch _relativerotation)) -45.0 1e+01) (.yaw _relativerotation)) false false))

(event Input|AxisEvents|InputAxisTurn
  (params (AxisValue :type Float%20%28single-precision%29))
  (Transformation|AddRelativeRotation (Variables|Default|GetCameraRoot) (Math|Rotator|MakeRotator 0.0 0.0 AxisValue) false false))

(fn ConstructionScript
  (|CallParentFunction))