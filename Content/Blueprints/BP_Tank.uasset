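; BP_Tank is a tank Blueprint that wires up its aiming, movement and status display components.
; On BeginPlay it passes the turret and barrel to TankAiming and the left and right tracks to TankMovement.
; It then casts the status widget's user widget to TankStatusUI and hands it a reference to itself.
; Each Tick it orients the status widget toward the camera.
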(event EventBeginPlay
  (Class|TankAimingComponent|Initialize (Variables|Default|GetTankAiming) (Variables|Default|GetTankTurret) (Variables|Default|GetTankBarrel))
  (Class|TankMovementComponent|Initialize (Variables|Default|GetTankMovement) (Variables|Default|GetLeftTrack) (Variables|Default|GetRightTrack))
  (bind _astank_status_ui (Utilities|Casting|CastToTankStatusUI (UserInterface|GetUserWidgetObject (Variables|Default|GetTankStatusWidget))))
  (Variables|/Game/Blueprints/UI/TankStatusUI.TankStatusUI_C|SetTank _astank_status_ui self))

(event EventTick
  (params (DeltaSeconds :type Float%20%28single-precision%29))
  (Class|TankStatusWidget|OrienttoCamera (Variables|Default|GetTankStatusWidget)))

(fn ConstructionScript)